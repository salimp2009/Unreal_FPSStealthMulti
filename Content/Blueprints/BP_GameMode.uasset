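; Game mode Blueprint that handles the end of a mission by showing the game-over screen.
; OnMissionCompleted waits briefly, clears all widgets, then creates WBP_GameOver and passes it the mission success result.
; An unconnected prototype finds an INT_SpectatingCamera actor and blends the instigator's view to the camera it returns, with that feature noted as moving to C++.
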(event EventBeginPlay)

(event EventTick
  (params (DeltaSeconds :type Float%20%28single-precision%29)))

(event EventOnMissionCompleted
  (params (InstigatorPawn :type Pawn%20Object%20Reference) (bMissionSuccess :type Boolean))
  (Utilities|FlowControl|Sequence
    (:then_0
      (Utilities|FlowControl|Delay 2.0)
      (Viewport|RemoveAllWidgets)
      (bind _returnvalue (UserInterface|CreateWidget "/Game/UI/WBP_GameOver.WBP_GameOver_C"))
      (UserInterface|Viewport|AddtoViewport _returnvalue 0)
      (Class|INTHUD|UpdateGameMission(Message) _returnvalue bMissionSuccess))))

(fn ConstructionScript)